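; AC_Detection is an actor component that detects what its owner, treated as the player, is looking at.
; On the eventDetection event, it finds the owner's camera component and line-traces along its forward vector, scaled by DistanceMultiplier, on a custom trace channel.
; It draws the trace for debugging and prints the hit actor's name, with no further handling of the result.
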(event Custom|eventDetection
  (bind _output_get (Variables|Default|SetPlayer (Components|GetOwner)))
  (bind _output_get_2 (Variables|Default|SetPlayer%20Camera (Actor|GetComponentbyClass _output_get "/Script/Engine.CameraComponent")))
  (Variables|Default|SetStart%20Location (Transformation|GetWorldLocation _output_get_2))
  (Variables|Default|SetEnd%20Location (+ (Transformation|GetWorldLocation _output_get_2) (* (Math|Vector|GetForwardVector (Transformation|GetWorldRotation _output_get_2)) (Variables|Default|GetDistance%20Multiplier))))
  (bind _outhit (Collision|LineTraceByChannel (Variables|Default|GetStart%20Location) (Variables|Default|GetEnd%20Location) "TraceTypeQuery4" false 0 "ForDuration"))
  (Development|PrintString (Utilities|GetDisplayName (.HitActor (Collision|BreakHitResult _outhit)))))