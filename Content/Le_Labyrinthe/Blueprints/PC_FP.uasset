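; PC_FP is the first-person player controller for the labyrinth game, translating Enhanced Input into character actions.
; On BeginPlay it adds the IMC_Perso mapping context.
; Move input drives the BP_FirstPersonCharacter, found by class lookup rather than the possessed pawn, along control-rotation right and forward vectors, while orbit input turns the view.
; Interact calls EventDetection on that character's ACDetection component.
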(event Input|EnhancedActionEvents|EnhancedInputActionIA_Move
  (params (ActionValue :type Vector%202D%20Structure) (ElapsedSeconds :type Float%20%28double-precision%29) (TriggeredSeconds :type Float%20%28double-precision%29) (InputAction :type Input%20Action%20Object%20Reference :default "/Game/Le_Labyrinthe/Inputs/IA_Move.IA_Move"))
  (bind _returnvalue (Pawn|GetControlRotation :!class /Script/Engine.Controller))
  ;[1 1 1] Movement
  (:Triggered
    (bind _returnvalue_2 (Actor|GetActorOfClass "/Game/Le_Labyrinthe/Blueprints/BP_FirstPersonCharacter.BP_FirstPersonCharacter_C"))
    (Pawn|Input|AddMovementInput _returnvalue_2 (Math|Vector|GetRightVector (Math|Rotator|MakeRotator (.roll _returnvalue) 0.0 (.yaw _returnvalue))) (.x ActionValue) false)
    (Pawn|Input|AddMovementInput _returnvalue_2 (Math|Vector|GetForwardVector (Math|Rotator|MakeRotator 0.0 0.0 (.yaw _returnvalue))) (.y ActionValue) false)))

(event Input|EnhancedActionEvents|EnhancedInputActionIA_Orbit
  (params (ActionValue :type Vector%202D%20Structure) (ElapsedSeconds :type Float%20%28double-precision%29) (TriggeredSeconds :type Float%20%28double-precision%29) (InputAction :type Input%20Action%20Object%20Reference :default "/Game/Le_Labyrinthe/Inputs/IA_Orbit.IA_Orbit"))
  ;[1 1 1] Camera
  (:Triggered
    (Class|PlayerController|AddYawInput (.x ActionValue))
    (Class|PlayerController|AddPitchInput (.y ActionValue))))

(event Input|EnhancedActionEvents|EnhancedInputActionIA_Interact
  (params (ActionValue :type Boolean) (ElapsedSeconds :type Float%20%28double-precision%29) (TriggeredSeconds :type Float%20%28double-precision%29) (InputAction :type Input%20Action%20Object%20Reference :default "/Game/Le_Labyrinthe/Inputs/IA_Interact.IA_Interact"))
  ;[1 1 1] Interact
  (:Started
    (bind _returnvalue (Actor|GetActorOfClass "/Game/Le_Labyrinthe/Blueprints/BP_FirstPersonCharacter.BP_FirstPersonCharacter_C"))
    (Default|EventDetection (Variables|/Game/Le_Labyrinthe/Blueprints/BP_FirstPersonCharacter.BP_FirstPersonCharacter_C|GetAC_Detection _returnvalue))))

(event EventBeginPlay
  (bind _returnvalue (PlayerController|LocalPlayerSubsystems|GetEnhancedInputLocalPlayerSubsystem))
  ;[0.5398 1 0.3401] SETUP
  (Utilities|IsValid _returnvalue
    (:Is%20Valid
      (Input|AddMappingContext _returnvalue "/Game/Le_Labyrinthe/Inputs/IMC_Perso.IMC_Perso" 0 "(bIgnoreAllPressedKeysUntilRelease=True,bForceImmediately=False)"))))

(fn ConstructionScript)